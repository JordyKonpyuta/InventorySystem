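; BP_TestBox is a test trigger box that takes 20 health or mana from the third-person character on overlap.
; The BoxType setting selects the stat, and the overlap event calls SetHealth or SetMana on the character in subtract mode.
; The construction script sets the text label to match the selected type.
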(event `self.Box.OnComponentBeginOverlap`
  (params (OverlappedComponent :type "PrimitiveComponent Object Reference") (OtherActor :type "Actor Object Reference") (OtherComp :type "PrimitiveComponent Object Reference") (OtherBodyIndex :type Integer) (bFromSweep :type Boolean) (SweepResult :type "HitResult Structure (by ref)"))
  (bind _asbp_third_person_character (cast `/Game/ThirdPerson/Blueprints/BP_ThirdPersonCharacter` OtherActor))
  (switch `/Game/Blueprints/E_BoxType` (`self.BoxType`)
    (:`NewEnumerator0`
      (`/Game/ThirdPerson/Blueprints/BP_ThirdPersonCharacter.SetHealth` _asbp_third_person_character 20.0 false))
    (:`NewEnumerator1`
      (`/Game/ThirdPerson/Blueprints/BP_ThirdPersonCharacter.SetMana` _asbp_third_person_character 20.0 false))))

(fn `UserConstructionScript`
  (switch `/Game/Blueprints/E_BoxType` (`self.BoxType`)
    (:`NewEnumerator0`
      (`TextRenderComponent.K2_SetText` (`self.TextRender`) (`|FormatText` "Health - 20")))
    (:`NewEnumerator1`
      (`TextRenderComponent.K2_SetText` (`self.TextRender`) (`|FormatText` "Mana - 20")))))